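; LightController_BP is a Blueprint that pulses a point light's intensity over time.
; Each Tick advances an angle at Tempo cycles per second and wraps it below 360 degrees.
; The sine of that angle, scaled by the Max-Min intensity range and offset by MinIntensity, sets the light's intensity.
; Because the sine is not remapped to 0-1, the value swings both above and below MinIntensity.
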(event EventBeginPlay)

(event EventTick
  (params (DeltaSeconds :type Float%20%28single-precision%29))
  (bind _output_get (Variables|Default|SetCurrentDeg (+ (Variables|Default|GetCurrentDeg) (* DeltaSeconds 3.6e+02 (Variables|Default|GetTempo)))))
  (while (>= _output_get 3.6e+02)
    (Variables|Default|SetCurrentDeg (- (Variables|Default|GetCurrentDeg) 3.6e+02)))
  (Rendering|Components|Light|SetIntensity (Variables|Default|GetPointLightComponent) (+ (* (Math|Trig|Sin(Radians) (Math|Trig|DegreesToRadians _output_get)) (- (Variables|Default|GetMaxIntensity) (Variables|Default|GetMinIntensity))) (Variables|Default|GetMinIntensity))))

(fn ConstructionScript)