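; Spawner actor that periodically drops Unko_BP objects into play at a random X offset around its mesh while generation is enabled.
; It pre-spawns an object pool off-screen at BeginPlay, and a looping timer moves instances from the pool to the active list.
; Destroy and DestroyAll recycle objects, though Destroy's index check (<= 0) skips all but the first active entry.
; Start, SetPause and the GameManager's game-over dispatch toggle generation.
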(event Custom|CreateEvent
  ;[1 1 1] 生成
  (if (Variables|Default|GetCanGenerate)
    (bind _created (プール|Create))
    (Transformation|SetActorTransform _created (Math|Transform|MakeTransform (+ (Transformation|GetWorldLocation (Variables|Debug|GetStaticMeshComponent)) (Math|Vector|MakeVector (Math|Conversions|ToFloat(Integer) (Math|Random|RandomIntegerinRange -300 300)) 0.0 0.0)) "0, 0, 0" "0.250000,0.250000,0.250000") false true)))

(event Custom|OnGameOver
  (Variables|Default|SetCanGenerate false))

(event EventBeginPlay
  (bind _manager (CallFunction|GetGameManager))
  ;[1 1 1] 初期化
  (Utilities|IsValid _manager
    (:Is%20Valid
      (EventDispatchers|BindEventtoGameOverEventDispatch _manager (delegate Custom|OnGameOver))
      (プール|InitializePool (Variables|設定|GetMaxUnkoPoolNum))
      (Utilities|Time|SetTimerbyEvent (delegate Custom|CreateEvent) 4.0 true))
    (:Is%20Not%20Valid
      (Development|PrintString "UnkoGeneratorBegin"))))

(event Collision|EventActorBeginOverlap
  (params (OtherActor :type Actor%20Object%20Reference)))

(event EventTick
  (params (DeltaSeconds :type Float%20%28single-precision%29)))

(fn ConstructionScript)

(fn InitializePool
  (params (UnkoNum :type Integer))
  (for _index (range 1 UnkoNum)
    (bind _returnvalue (Game|SpawnActorfromClass "/Game/Blueprints/Items/Unko_BP.Unko_BP_C" (Math|Transform|MakeTransform "0.000000,1000.000000, 0") "Undefined" 0 0))
    (Utilities|Array|Add (Variables|プール|GetUnkoPool) _returnvalue))
  (return))

(fn Create
  (bind _unkopool (Variables|プール|GetUnkoPool))
  (bind _usedobjects (Variables|プール|GetUsedObjects))
  (bind _returnvalue (Utilities|Array|LastIndex _usedobjects))
  (bind _output (Utilities|Array|Get(acopy) _usedobjects _returnvalue))
  (if (> (Utilities|Array|Length (Variables|プール|GetUnkoPool)) 0)
    (Utilities|Array|Add _usedobjects (Utilities|Array|Get(acopy) _unkopool))
    (Utilities|Array|RemoveIndex _unkopool)
    (Default|OnCreate _output)
    (return _output)
    (else
      (Development|PrintString "Error : オブジェクトプールが足りません")
      (return 0))))

(fn Destroy
  (params (DestroyObj :type Unko%20BP%20Object%20Reference))
  (bind _usedobjects (Variables|プール|GetUsedObjects))
  (bind _usedobjects_2 (Variables|プール|GetUsedObjects))
  (bind _returnvalue (Utilities|Array|FindItem _usedobjects DestroyObj))
  (Default|OnDestroy DestroyObj)
  (if (<= _returnvalue 0)
    (Utilities|Array|Add (Variables|プール|GetUnkoPool) (Utilities|Array|Get(acopy) _usedobjects_2 _returnvalue))
    (Utilities|Array|RemoveIndex _usedobjects_2 _returnvalue)))

(fn GetActiveObjects
  (return (Variables|プール|GetUsedObjects)))

(fn Start
  (Variables|Default|SetCanGenerate true))

(fn SetPause
  (params (PauseEnabled :type Boolean))
  (Variables|Default|SetCanGenerate (not PauseEnabled))
  (for _array_element (Variables|プール|GetUsedObjects)
    (Default|SetPause _array_element PauseEnabled)))

(fn DestroyAll
  (for _array_element (Variables|プール|GetUsedObjects)
    (Default|OnDestroy _array_element)
    (Utilities|Array|Add (Variables|プール|GetUnkoPool) _array_element))
  (Utilities|Array|Clear (Variables|プール|GetUsedObjects)))