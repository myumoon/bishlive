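; Manager for a group of Otaku characters that makes them jump highest near the touched point, forming a hill shape along X.
; Each Tick it deprojects the mouse position and line-traces it against the TouchCollision brush.
; An ease-in-out falloff over X distance scales each Otaku's max jump offset, which is zero without a hit.
; SetPause forwards to every Otaku, and GetOtakuIndexByXPos is an unimplemented stub.
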(event EventBeginPlay)

(event Collision|EventActorBeginOverlap
  (params (OtherActor :type Actor%20Object%20Reference)))

(event EventTick
  (params (DeltaSeconds :type Float%20%28single-precision%29))
  (bind (_location _istouched) (CallFunction|GetTouchLocation))
  (for _array_element (Variables|初期化|GetOtakus)
    (if _istouched
      (bind _influence (CallFunction|CalcTouchInfluence (.X (Math|Vector|BreakVector _location)) _array_element))
      (Default|SetMaxJumpOffset _array_element (* _influence (Variables|初期化|GetJumpHeight)))
      (else
        (Default|SetMaxJumpOffset _array_element 0.0)))))

(fn ConstructionScript)

(fn GetTouchLocation
  (bind _returnvalue (Game|GetPlayerController 0))
  (bind (_locationx _locationy) (Game|Player|GetMousePosition _returnvalue))
  (bind _returnvalue_2 (Math|Vector2D|MakeVector2D _locationx _locationy))
  (bind (_worldposition _worlddirection) (Class|GameplayStatics|DeprojectScreentoWorld _returnvalue _returnvalue_2))
  (bind (_hitlocation _hitnormal _bonename _outhit _returnvalue_3) (Collision|LineTraceComponent (Variables|/Script/Engine.Brush|GetBrushComponent (Variables|初期化|GetTouchCollision)) _worldposition (+ _worldposition (* _worlddirection 1000)) true false))
  (return _hitlocation _returnvalue_3))

(fn GetOtakuIndexbyXPos
  (params (PosX :type Float%20%28single-precision%29))
  (return 0.0))

(fn CalcTouchInfluence
  (params (TouchedPosX :type Float%20%28single-precision%29) (Otaku :type Otaku%20BP%20Object%20Reference))
  (bind _returnvalue (Transformation|GetActorLocation Otaku))
  (bind _x (Math|Vector|BreakVector _returnvalue))
  (bind _returnvalue_2 (- TouchedPosX _x))
  (bind _returnvalue_3 (Math|Float|Absolute(Float) _returnvalue_2))
  (if (<= (- (Variables|初期化|GetTouchInfluenceLength) _returnvalue_3) 0.0) ; 影響範囲外か？
    (return 0.0)
    (else
      (return (Class|KismetMathLibrary|FInterpEaseinOut 0.0 1.0 (- 1.0 (/ _returnvalue_3 (Variables|初期化|GetTouchInfluenceLength))) 2.0)))))

(fn SetPause
  (params (PauseEnabled :type Boolean))
  (for _array_element (Variables|初期化|GetOtakus)
    (Default|SetPause _array_element PauseEnabled)))