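; Otaku character actor that hops while the mouse cursor is over it and drops back when the cursor leaves.
; Tick line-traces from the deprojected mouse position against the TouchBox component.
; Paired DoOnce nodes re-arm each other, so each hover change fires JumpEvent or JumpEndEvent once.
; These play or reverse a timeline that offsets the actor from its BeginPlay location.
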(event EventBeginPlay
  (Variables|アニメーション|SetBaseLocation (Transformation|GetActorLocation)))

(event Collision|EventActorBeginOverlap
  (params (OtherActor :type Actor%20Object%20Reference)))

(event EventTick
  (params (DeltaSeconds :type Float%20%28single-precision%29))
  (if (ヒット|IsTouched)
    (Utilities|FlowControl|DoOnce false :!label _label
      (:Completed
        (Utilities|FlowControl|Sequence
          (:then_0
            (CallFunction|JumpEvent))
          (:then_1
            (goto _label_2 Reset)))))
    (else
      (Utilities|FlowControl|DoOnce false :!label _label_2
        (:Completed
          (Utilities|FlowControl|Sequence
            (:then_0
              (CallFunction|JumpEndEvent))
            (:then_1
              (goto _label Reset))))))))

(event Custom|JumpEvent
  (bind _新規track_0 (Timeline|タイムライン_0 Play)
    (:Update
      (Transformation|SetActorLocation (+ _新規track_0 (Variables|アニメーション|GetBaseLocation)) false false))))

(event Custom|JumpEndEvent
  (bind _新規track_0 (Timeline|タイムライン_0 Reverse)
    (:Update
      (Transformation|SetActorLocation (+ _新規track_0 (Variables|アニメーション|GetBaseLocation)) false false))))

(fn ConstructionScript)

(fn IsTouched
  (bind _returnvalue (Game|GetPlayerController 0))
  (bind (_locationx _locationy) (Game|Player|GetMousePosition _returnvalue))
  (bind _returnvalue_2 (Math|Vector2D|MakeVector2D _locationx _locationy))
  (bind (_worldposition _worlddirection) (Class|GameplayStatics|DeprojectScreentoWorld _returnvalue _returnvalue_2))
  (bind _returnvalue_3 (Collision|LineTraceComponent (Variables|Default|GetTouchBox) _worldposition (+ _worldposition (* _worlddirection 1000)) true false))
  (return _returnvalue_3))

(fn Jump)