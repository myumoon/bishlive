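; BishUtil is a utility Blueprint that gives access to the game's manager actors: GameManager, UnkoGenerator, OtakuManager and UIManager.
; A shared GetInstanceOf helper searches the world by class with GetAllActorsOfClass and returns the first match, printing "Error" if none exists.
; Each getter casts that helper's result to its manager type, so every call repeats the actor search without caching.
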(fn GetGameManager
  (bind _asgame_manager (Utilities|Casting|CastToGameManager (CallFunction|GetInstanceOf 0 (LocalVariables|Get__WorldContext))))
  (return _asgame_manager))

(fn GetInstanceOf
  (params (Class :type Actor%20Class%20Reference))
  (bind _outactors (Actor|GetAllActorsOfClass (LocalVariables|Get__WorldContext) Class))
  (if (> (Utilities|Array|Length _outactors) 0)
    (return (Utilities|Array|Get(acopy) _outactors))
    (else
      (Development|PrintString 0 "Error")
      (return 0))))

(fn GetUnkoManager
  (bind _asunko_generator (Utilities|Casting|CastToUnkoGenerator (CallFunction|GetInstanceOf "/Game/Blueprints/Items/UnkoGenerator.UnkoGenerator_C")))
  (return _asunko_generator))

(fn GetOtakuManager
  (bind _asotaku_manager (Utilities|Casting|CastToOtakuManager (CallFunction|GetInstanceOf "/Game/Blueprints/Characters/OtakuManager.OtakuManager_C")))
  (return _asotaku_manager))

(fn GetUIManager
  (bind _asuimanager (Utilities|Casting|CastToUIManager (CallFunction|GetInstanceOf "/Game/Blueprints/UI/UIManager.UIManager_C")))
  (return _asuimanager))