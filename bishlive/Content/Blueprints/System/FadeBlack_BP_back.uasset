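; FadeBlack_BP_back is an actor that fades a black material in and out by animating its Alpha parameter.
; The construction script creates a dynamic instance of Fade_black_Mat on RenderComponent, which BeginPlay caches.
; FadeIn and FadeOut set direction and duration, then Tick interpolates Alpha linearly, scaled by MaxAlpha, and prints the ratio.
; IsFading is never cleared here, and CalcRate is not called within this Blueprint.
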(event EventBeginPlay
  (bind _asmaterial_instance_dynamic (Utilities|Casting|CastToMaterialInstanceDynamic (Rendering|Material|GetMaterial (Variables|Default|GetRenderComponent) 0)))
  (Variables|Default|SetFadeMaterial _asmaterial_instance_dynamic))

(event Collision|EventActorBeginOverlap
  (params (OtherActor :type Actor%20Object%20Reference)))

(event EventTick
  (params (DeltaSeconds :type Float%20%28single-precision%29))
  (bind _fadetime (Variables|Default|GetFadeTime))
  (if (Variables|Default|GetIsFading)
    (bind _output_get (Variables|Default|SetCurrentTime (Math|Float|Min(Float) (+ DeltaSeconds (Variables|Default|GetCurrentTime)) _fadetime)))
    (if (< (Variables|Default|GetFrom) (Variables|Default|GetTo))
      (Development|PrintString (Utilities|String|ToString(Float) (/ _output_get _fadetime)))
      (Rendering|Material|SetScalarParameterValue (Variables|Default|GetFadeMaterial) "Alpha" (* (Variables|Default|GetMaxAlpha) (/ _output_get _fadetime)) :!class /Script/Engine.MaterialInstanceDynamic)
      (else
        (Development|PrintString (Utilities|String|ToString(Float) (- 1.0 (/ _output_get _fadetime))))
        (Rendering|Material|SetScalarParameterValue (Variables|Default|GetFadeMaterial) "Alpha" (* (- 1.0 (/ _output_get _fadetime)) (Variables|Default|GetMaxAlpha)) :!class /Script/Engine.MaterialInstanceDynamic)))))

(fn ConstructionScript
  (Rendering|Material|CreateDynamicMaterialInstance (Variables|Default|GetRenderComponent) 0 "/Game/2D/Fade/fade_black_Mat.fade_black_Mat" :!class /Script/Engine.PrimitiveComponent))

(fn Fadein
  (params (InTime :type Float%20%28single-precision%29))
  (Variables|Default|SetFadeTime InTime)
  (Variables|Default|SetFrom 1.0)
  (Variables|Default|SetTo 0.0)
  (Variables|Default|SetCurrentTime 0.0)
  (Variables|Default|SetIsFading true))

(fn FadeOut
  (params (OutTime :type Float%20%28single-precision%29))
  (Variables|Default|SetFadeTime OutTime)
  (Variables|Default|SetFrom 0.0)
  (Variables|Default|SetTo 1.0)
  (Variables|Default|SetCurrentTime 0.0)
  (Variables|Default|SetIsFading true))

(fn CalcRate
  (bind _currenttime (Variables|Default|GetCurrentTime))
  (bind _to (Variables|Default|GetTo))
  (bind _from (Variables|Default|GetFrom))
  (bind _returnvalue (- _to _from))
  (bind _returnvalue_2 (/ _currenttime _returnvalue))
  (bind _returnvalue_3 (- 1.0 _returnvalue_2))
  (if (< _returnvalue_2 0.0)
    (return (* (Variables|Default|GetMaxAlpha) _returnvalue_3))
    (else
      (return (* _returnvalue_3 (Variables|Default|GetMaxAlpha))))))