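; Main game camera that keeps depth-of-field focus on the member manager's current member.
; Each Tick sets the focal distance by projecting the camera-to-member offset, with member X zeroed, onto the camera's forward vector.
; ChangeModeGameOver applies fixed depth-of-field settings with far blur only.
; IsInGame is set on BeginPlay but never checked, so Tick keeps overriding the game-over focal distance while it runs.
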(event EventBeginPlay
  (Variables|Default|SetIsInGame true))

(event Collision|EventActorBeginOverlap
  (params (OtherActor :type Actor%20Object%20Reference)))

(event EventTick
  (params (DeltaSeconds :type Float%20%28single-precision%29))
  (bind _manager (CallFunction|GetMemberManager))
  (bind _cameracomponent (Variables|CameraActor|GetCameraComponent))
  (bind _currentmember (Variables|/Game/Blueprints/Members/MemberManager.MemberManager_C|GetCurrentMember _manager))
  (bind _returnvalue (Transformation|GetActorLocation _currentmember))
  (bind (_x _y _z) (Math|Vector|BreakVector _returnvalue))
  (Variables|/Script/Engine.CameraComponent|SetPostProcessSettings _cameracomponent (Utilities|Struct|MakePostProcessSettings (.DepthOfFieldFstop (Utilities|Struct|BreakPostProcessSettings (Variables|/Script/Engine.CameraComponent|GetPostProcessSettings _cameracomponent))) (- (Math|Vector|DotProduct (- (Math|Vector|MakeVector 0.0 _y _z) (Transformation|GetActorLocation)) (Transformation|GetActorForwardVector)) 1.0) (.DepthOfFieldDepthBlurAmount (Utilities|Struct|BreakPostProcessSettings (Variables|/Script/Engine.CameraComponent|GetPostProcessSettings _cameracomponent))) (.DepthOfFieldDepthBlurRadius (Utilities|Struct|BreakPostProcessSettings (Variables|/Script/Engine.CameraComponent|GetPostProcessSettings _cameracomponent))) (.DepthOfFieldFocalRegion (Utilities|Struct|BreakPostProcessSettings (Variables|/Script/Engine.CameraComponent|GetPostProcessSettings _cameracomponent))) (.DepthOfFieldNearTransitionRegion (Utilities|Struct|BreakPostProcessSettings (Variables|/Script/Engine.CameraComponent|GetPostProcessSettings _cameracomponent))) (.DepthOfFieldFarTransitionRegion (Utilities|Struct|BreakPostProcessSettings (Variables|/Script/Engine.CameraComponent|GetPostProcessSettings _cameracomponent))) (.DepthOfFieldScale (Utilities|Struct|BreakPostProcessSettings (Variables|/Script/Engine.CameraComponent|GetPostProcessSettings _cameracomponent))) (.DepthOfFieldMaxBokehSize (Utilities|Struct|BreakPostProcessSettings (Variables|/Script/Engine.CameraComponent|GetPostProcessSettings _cameracomponent))) (.DepthOfFieldNearBlurSize (Utilities|Struct|BreakPostProcessSettings (Variables|/Script/Engine.CameraComponent|GetPostProcessSettings _cameracomponent))) (.DepthOfFieldFarBlurSize (Utilities|Struct|BreakPostProcessSettings (Variables|/Script/Engine.CameraComponent|GetPostProcessSettings _cameracomponent))))))

(fn ConstructionScript)

(fn ChangeModeGameOver
  (bind _cameracomponent (Variables|CameraActor|GetCameraComponent))
  (Variables|/Script/Engine.CameraComponent|SetPostProcessSettings _cameracomponent (Utilities|Struct|MakePostProcessSettings (.DepthOfFieldFstop (Utilities|Struct|BreakPostProcessSettings (Variables|/Script/Engine.CameraComponent|GetPostProcessSettings _cameracomponent))) 1.3e+03 (.DepthOfFieldDepthBlurAmount (Utilities|Struct|BreakPostProcessSettings (Variables|/Script/Engine.CameraComponent|GetPostProcessSettings _cameracomponent))) (.DepthOfFieldDepthBlurRadius (Utilities|Struct|BreakPostProcessSettings (Variables|/Script/Engine.CameraComponent|GetPostProcessSettings _cameracomponent))) 1e+03 5e+02 1.0 0.0 3e+01 0.0 3e+01)))