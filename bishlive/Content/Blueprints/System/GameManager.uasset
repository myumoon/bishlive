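; Game manager actor that runs the match flow as members take turns diving and handles their special moves.
; Tick drives a state machine from start wait through dive, timed play and return, advancing members until game clear.
; Game over, triggered externally, dispatches an event and restarts through BishGameMode after a delay.
; Specials pause the managers and fade out for a UI cut-in, then dispatchers chain the member's special into unpause, Unko cleanup and fade-in.
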(event Custom|OnSpecialUIEnd
  (bind _manager (CallFunction|GetMemberManager))
  (bind _newparam (Default|GetCurrentMember _manager))
  (EventDispatchers|AssignSpecialEndDispatcher _newparam (delegate Custom|OnSpecialMemberEnd))
  (Default|StartSpecial _newparam))

(event Custom|OnSpecialMemberEnd
  (bind _manager (CallFunction|GetUnkoManager))
  (EventDispatchers|UnbindallEventsfromSpecialEndDispatcher (Default|GetCurrentMember (CallFunction|GetMemberManager)))
  (Default|SetPause (CallFunction|GetOtakuManager) false)
  (Default|SetPauseasSpecial (CallFunction|GetMemberManager) false)
  (Default|SetPause _manager false)
  (Default|DestroyAll _manager)
  (Default|Fadein (CallFunction|GetFader) 0.5))

(event EventBeginPlay
  (EventDispatchers|AssignSpecialEndDispatcher (CallFunction|GetUIManager) (delegate Custom|OnSpecialUIEnd))
  (Default|SetPause (CallFunction|GetUnkoManager) false))

(event Collision|EventActorBeginOverlap
  (params (OtherActor :type Actor%20Object%20Reference)))

(event EventTick
  (params (DeltaSeconds :type Float%20%28single-precision%29))
  (bind _nextstate (Variables|Default|GetNextState))
  (Variables|Default|SetStateInitialize (Utilities|Enum|NotEqual(Enum) (Variables|Default|GetGameState) _nextstate))
  (bind _output_get (Variables|Default|SetGameState _nextstate))
  (switch Utilities|FlowControl|Switch|SwitchonGameState _output_get
    (:NewEnumerator0
      (CallFunction|UpdateStateStartWait (Variables|Default|GetStateInitialize) (stale Input|KeyboardEvents|A _output_get)))
    (:NewEnumerator1
      (CallFunction|UpdateStateStartEvent (Variables|Default|GetStateInitialize)))
    (:NewEnumerator5
      (CallFunction|UpdateStateDivePerformane (Variables|Default|GetStateInitialize)))
    (:NewEnumerator2
      (CallFunction|UpdateStateDive (Variables|Default|GetStateInitialize)))
    (:NewEnumerator3
      (CallFunction|UpdateStateGame (Variables|Default|GetStateInitialize) DeltaSeconds))
    (:NewEnumerator4
      (CallFunction|UpdateStateReturn (Variables|Default|GetStateInitialize) DeltaSeconds))
    (:NewEnumerator6
      (CallFunction|UpdateStateGameOver (Variables|Default|GetStateInitialize) DeltaSeconds))
    (:NewEnumerator7
      (CallFunction|UpdateStateGameClear (Variables|Default|GetStateInitialize)))))

(event Input|KeyboardEvents|A
  (params (Key :type Key%20Structure :default "AnyKey"))
  (bind _manager (CallFunction|GetMemberManager))
  (bind _newparam (Default|GetCurrentMember _manager))
  (:Pressed
    (bind _output_get (Variables|Default|SetCanStart true))
    (Utilities|IsValid _newparam
      (:Is%20Valid
        (Default|StartDive _newparam))
      (:Is%20Not%20Valid
        (Development|PrintString "Hello")))))

(fn ConstructionScript
  (bind _output_get (Variables|Default|SetGameState "NewEnumerator0"))
  (Variables|Default|SetNextState _output_get))

(fn SendGameOverEvent
  (Variables|Default|SetNextState "NewEnumerator6"))

(fn StartSpecial
  (params (Member :type MemberType%20Enum))
  (Utilities|FlowControl|Sequence
    (:then_0
      ;[1 1 1] ここで設定したのがUIから参照される
      (bind _outactors (Actor|GetAllActorsOfClass "/Game/Blueprints/UI/Special/SpecialCutImgBinder.SpecialCutImgBinder_C"))
      (Default|SetNextMember (Utilities|Array|Get(acopy) _outactors) Member))
    (:then_1
      ;[1 1 1] 再生
      (bind _foundwidgets (Widget|GetAllWidgetsOfClass "/Game/Blueprints/UI/Special/SpecialCutWiddget_BP.SpecialCutWiddget_BP_C" true))
      (bind _asspecial_cut_widdget_bp (Utilities|Casting|CastToSpecialCutWiddget_BP (Utilities|Array|Get(acopy) _foundwidgets)))
      (UserInterface|Animation|PlayAnimation _asspecial_cut_widdget_bp (Variables|/Game/Blueprints/UI/Special/SpecialCutWiddget_BP.SpecialCutWiddget_BP_C|GetCut _asspecial_cut_widdget_bp) 0.0 1 "Forward" 1.0))
    (:then_2
      ;[1 1 1] ポーズ
      (Default|SetPause (CallFunction|GetOtakuManager) true)
      (Default|SetPauseasSpecial (CallFunction|GetMemberManager) true)
      (Default|SetPause (CallFunction|GetUnkoManager) true))
    (:then_3
      (Default|OnBeginSpecialCut (Variables|/Game/Blueprints/Members/MemberManager.MemberManager_C|GetCurrentMember (CallFunction|GetMemberManager))))
    (:then_4
      (Default|FadeOut (CallFunction|GetFader) 0.5))))

(fn GetDivePoint
  (bind _divepoint (Variables|Default|GetDivePoint))
  (Utilities|IsValid _divepoint
    (:Is%20Valid
      (return (Transformation|GetActorLocation _divepoint)))
    (:Is%20Not%20Valid
      (return "0, 0, 0"))))

(fn UpdateStateStartWait
  (params (Initialize :type Boolean) (CanStart :type Boolean))
  (if CanStart
    (Variables|Default|SetNextState "NewEnumerator1")))

(fn UpdateStateStartEvent
  (params (Initialize :type Boolean))
  (Variables|Default|SetNextState "NewEnumerator5"))

(fn UpdateStateDivePerformane
  (params (Initialize :type Boolean))
  (if Initialize
    ;[1 1 1] todo : ここで演出を入れる
    (Variables|Default|SetNextState "NewEnumerator2")))

(fn UpdateStateDive
  (params (Initialize :type Boolean))
  (if (Utilities|Enum|Equal(Enum) (Variables|/Game/Blueprints/Members/MemberBase_BP.MemberBase_BP_C|GetCurrentState (Default|GetCurrentMember (CallFunction|GetMemberManager))) "NewEnumerator3")
    (Variables|Default|SetNextState "NewEnumerator3")))

(fn UpdateStateGame
  (params (Initialize :type Boolean) (DeltaTime :type Float%20%28single-precision%29))
  (Utilities|FlowControl|Sequence
    (:then_0
      (if Initialize
        (Variables|Default|SetWaitTime 0.0)))
    (:then_1
      (bind _output_get (Variables|Default|SetWaitTime (+ DeltaTime (Variables|Default|GetWaitTime))))
      (if (>= _output_get (Variables|Default|GetGameTime))
        (Variables|Default|SetNextState "NewEnumerator4")))))

(fn UpdateStateReturn
  (params (Initialize :type Boolean) (DeltaTime :type Float%20%28single-precision%29))
  (Utilities|FlowControl|Sequence
    (:then_0
      ;[1 1 1] 初期化
      (if Initialize
        (Default|ReturnStage (Default|GetCurrentMember (CallFunction|GetMemberManager)))))
    (:then_1
      (if (Utilities|Enum|Equal(Enum) (Default|GetCurrentState (Default|GetCurrentMember (CallFunction|GetMemberManager))) "NewEnumerator0")
        (if (Default|IsLastMember (CallFunction|GetMemberManager))
          (Variables|Default|SetNextState "NewEnumerator7")
          (else
            (Variables|Default|SetNextState "NewEnumerator5")
            (Default|ChangeNextMember (CallFunction|GetMemberManager))))))))

(fn UpdateStateGameOver
  (params (Initialize :type Boolean) (DeltaTime :type Float%20%28single-precision%29))
  (Utilities|FlowControl|Sequence
    (:then_0
      (if Initialize
        (Default|CallGameOverEventDispatch)
        (Variables|Default|SetWaitTime 0.0)))
    (:then_1
      (bind _output_get (Variables|Default|SetWaitTime (+ DeltaTime (Variables|Default|GetWaitTime))))
      (if (>= _output_get (Variables|Default|GetGameOverWaitTime))
        (Variables|Default|SetNextState "NewEnumerator0")
        (bind _asbish_game_mode (Utilities|Casting|CastToBishGameMode (Game|GetGameMode)))
        (Development|PrintString "RestartGame!!" false)
        (Class|GameMode|RestartGame _asbish_game_mode)))))

(fn UpdateStateGameClear
  (params (Initialize :type Boolean)))