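; MemberManager is an actor Blueprint that tracks which entry in its Members array is current, apparently for a sequence of divers.
; Construction selects the first member, and ChangeNextMember advances through the array without wrapping at the end.
; ChangeNextDiver resets to the first member and starts its dive.
; SetPauseAsSpecial pauses everyone except the current member, or unpauses all members when disabled.
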(event EventBeginPlay)

(event Collision|EventActorBeginOverlap
  (params (OtherActor :type Actor%20Object%20Reference)))

(event EventTick
  (params (DeltaSeconds :type Float%20%28single-precision%29)))

(fn ConstructionScript
  (Variables|Default|SetCurrentMember (Utilities|Array|Get(acopy) (Variables|メンバー|GetMembers))))

(fn ChangeNextMember
  (bind _members (Variables|メンバー|GetMembers))
  (if (> (Utilities|Array|Length _members) (+ (Utilities|Array|FindItem _members (Variables|Default|GetCurrentMember)) 1))
    (bind _output_get (Variables|Default|SetCurrentMember (Utilities|Array|Get(acopy) _members (+ (Utilities|Array|FindItem _members (Variables|Default|GetCurrentMember)) 1))))
    (return _output_get)
    (else
      (return 0))))

(fn SetPauseasSpecial
  (params (PauseEnabled :type Boolean))
  (if PauseEnabled
    (for _array_element (Variables|メンバー|GetMembers)
      (if (!= _array_element (CallFunction|GetCurrentMember))
        (Default|SetPause _array_element true)))
    (else
      (for _array_element_2 (Variables|メンバー|GetMembers)
        (Default|SetPause _array_element_2 false)))))

(fn GetCurrentMember
  (return (Variables|Default|GetCurrentMember)))

(fn ChangeNextDiver
  (bind _output_get (Variables|Default|SetCurrentMember (Utilities|Array|Get(acopy) (Variables|メンバー|GetMembers))))
  (Default|StartDive _output_get))