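; Base Paper2D stage member that dives into the otaku crowd, bounces there, and ends the game on touching Unko outside a special.
; Timelines arc it between stage and dive point, switching plane constraints, physics and render priority; near otaku, timed random upward impulses keep it moving.
; Its special visits each active Unko in turn using a front material.
; A small flipbook state machine lets the Togetoge hop loop finish before switching animations.
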(event OnComponentHit(CapsuleComponent)
  (params (HitComponent :type Primitive%20Component%20Object%20Reference) (OtherActor :type Actor%20Object%20Reference) (OtherComp :type Primitive%20Component%20Object%20Reference) (NormalImpulse :type Vector :default "0, 0, 0") (Hit :type Hit%20Result%20Structure%20%28by%20ref%29))
  ;[1 1 1] オタクと当たった
  (Utilities|Casting|CastTootaku_BP OtherActor)
  (Utilities|FlowControl|Sequence
    (:then_0
      ;[1 1 1] エフェクトを出す
      (bind _returnvalue (Effects|SpawnEmitteratLocation (Variables|Default|GetCrashOtakuParticle) (- (.ImpactPoint (Collision|BreakHitResult Hit)) "0, 0,25.000000")))
      (Rendering|SetTranslucentSortPriority _returnvalue (CallFunction|GetRenderPriority "NewEnumerator6")))))

(event OnComponentBeginOverlap(CapsuleComponent)
  (params (OverlappedComponent :type Primitive%20Component%20Object%20Reference) (OtherActor :type Actor%20Object%20Reference) (OtherComp :type Primitive%20Component%20Object%20Reference) (OtherBodyIndex :type Integer) (bFromSweep :type Boolean) (SweepResult :type Hit%20Result%20Structure%20%28by%20ref%29))
  ;[1 1 1] うんこに当たったらゲームオーバー
  (if (not (Variables|必殺技|GetIsPlaySpecial))
    (Utilities|IsValid OtherActor
      (:Is%20Valid
        (if (Actor|ActorHasTag OtherActor "Unko")
          (bind _outactors (Actor|GetAllActorsOfClass "/Game/Blueprints/System/GameManager.GameManager_C"))
          (Default|GameOver (Utilities|Array|Get(acopy) _outactors)))))))

(event OnComponentEndOverlap(AutoMoveOverwrap)
  (params (OverlappedComponent :type Primitive%20Component%20Object%20Reference) (OtherActor :type Actor%20Object%20Reference) (OtherComp :type Primitive%20Component%20Object%20Reference) (OtherBodyIndex :type Integer))
  ;[1 1 1] オタクと一定距離内の場合に勝手に動くようにする
  (Utilities|Casting|CastTootaku_BP OtherActor)
  (Variables|難易度|SetIsUpdateAutoMoveCount false))

(event OnComponentBeginOverlap(AutoMoveOverwrap)
  (params (OverlappedComponent :type Primitive%20Component%20Object%20Reference) (OtherActor :type Actor%20Object%20Reference) (OtherComp :type Primitive%20Component%20Object%20Reference) (OtherBodyIndex :type Integer) (bFromSweep :type Boolean) (SweepResult :type Hit%20Result%20Structure%20%28by%20ref%29))
  ;[1 1 1] オタクと一定距離内の場合に勝手に動くようにする
  (Utilities|Casting|CastTootaku_BP OtherActor)
  (Variables|難易度|SetIsUpdateAutoMoveCount true))

(event Custom|Special_MoveTo
  (params (To :type Actor%20Object%20Reference))
  (bind _returnvalue (Transformation|GetActorLocation To))
  ;[1 1 1] スペシャル状態遷移
  (Variables|Default|SetMoveBasePos (Transformation|GetActorLocation))
  (bind _rate (Timeline|SpecialMoveToTimeline PlayFromStart)
    (:Update
      (Development|PrintString (Utilities|String|ToString(Text) (Utilities|Text|FormatText "target {1}, current {2}" (Utilities|Text|ToText(String) _returnvalue) (Utilities|Text|ToText(String) (* (- _returnvalue (Variables|Default|GetMoveBasePos)) _rate)))) false)
      (Transformation|SetActorLocation (Math|Vector|MakeVector (.X (Math|Vector|BreakVector (+ (Variables|Default|GetMoveBasePos) (* (- _returnvalue (Variables|Default|GetMoveBasePos)) _rate)))) (.Y (Math|Vector|BreakVector (Transformation|GetActorLocation))) (.Z (Math|Vector|BreakVector (+ (Variables|Default|GetMoveBasePos) (* (- _returnvalue (Variables|Default|GetMoveBasePos)) _rate))))) false false))
    (:Finished
      (CallFunction|SpecialAction)
      (Transformation|SetActorLocation _returnvalue false true))))

(event Custom|OnStartDive
  ;[1 1 1] ステージからダイブ
  (Rendering|SetTranslucentSortPriority (Variables|Default|GetPaperFlipbook) (CallFunction|GetRenderPriority "NewEnumerator0"))
  (Class|PrimitiveComponent|SetConstraintMode (Variables|Collision|GetCapsuleComponent) "Default") ; 手前に動けるようにするためにデフォルトに戻す
  (Variables|Default|SetMoveBasePos (Transformation|GetActorLocation))
  (CallFunction|OnAnimChange "NewEnumerator5")
  (Utilities|FlowControl|Delay 0.2)
  (bind (_direction _yrate _height) (Timeline|MoveToDivePointXZ PlayFromStart)
    (:Update
      (bind _returnvalue (CallFunction|UpdateDivingPosition _yrate _height (Default|GetDivePoint (CallFunction|GetGameManager))))
      (Transformation|SetActorLocation _returnvalue false true))
    (:Finished
      (Transformation|SetActorLocation (Default|GetDivePoint (CallFunction|GetGameManager)) false true)
      (CallFunction|SetDiveMode))))

(event Custom|Special_Action
  ;[1 1 1] スペシャル状態遷移
  (CallFunction|OnAnimChange "NewEnumerator2")
  (Utilities|FlowControl|Delay 0.8)
  (CallFunction|OnAnimChange "NewEnumerator0")
  (CallFunction|SpecialWait))

(event Custom|Special_Wait
  ;[1 1 1] スペシャル状態遷移
  (Utilities|FlowControl|Delay 0.8)
  (CallFunction|SpecialSetNext))

(event Custom|Special_SetNext
  ;[1 1 1] スペシャル状態遷移
  (bind _result (Math|Integer|IncrementInt (Variables|必殺技|GetCurrentTargetIndex))
    (:%20%20
      (if (< _result (Utilities|Array|Length (Variables|必殺技|GetTargets)))
        (CallFunction|SpecialMoveto (Utilities|Array|Get(acopy) (Variables|必殺技|GetTargets) _result))
        (else
          (CallFunction|EndSpecial)
          (Default|CallSpecialEndDispatcher))))))

(event Custom|OnReturnStage
  (bind _stagepos (Variables|Default|GetStagePos))
  ;[1 1 1] ステージに戻る
  (Class|PrimitiveComponent|SetConstraintMode (Variables|Collision|GetCapsuleComponent) "Default") ; 手前に動けるようにするためにデフォルトに戻す
  (Variables|Default|SetMoveBasePos (Transformation|GetActorLocation))
  (Utilities|FlowControl|Delay 0.2)
  (bind (_direction _yrate _height) (Timeline|タイムライン_0 PlayFromStart)
    (:Update
      (bind _returnvalue (CallFunction|UpdateDivingPosition _yrate _height _stagepos))
      (Transformation|SetActorLocation _returnvalue false true)
      (CallFunction|UpdateDivingRotation (Transformation|GetActorRotation)))
    (:Finished
      (Transformation|SetActorLocation _stagepos false true)
      (Transformation|SetActorRotation "0, 0, 0")
      (CallFunction|SetStageMode))))

(event Custom|OnBeginSpecial)

(event Custom|OnGameOver
  ;[1 1 1] 初期化
)

(event EventBeginPlay
  ;[1 1 1] 初期化
  (bind _outactors (Actor|GetAllActorsOfClass "/Game/Blueprints/System/GameManager.GameManager_C"))
  (EventDispatchers|BindEventtoGameOverEventDispatch (Utilities|Array|Get(acopy) _outactors) (delegate Custom|OnGameOver))
  (CallFunction|OnAnimEnter)
  (CallFunction|OnAnimChange "NewEnumerator1")
  (Rendering|SetTranslucentSortPriority (Variables|Default|GetPaperFlipbook) (CallFunction|GetRenderPriority "NewEnumerator3")))

(event EventTick
  (params (DeltaSeconds :type Float%20%28single-precision%29))
  (if (not (Variables|Default|GetPauseEnabled))
    (switch Utilities|FlowControl|Switch|SwitchonMemberState (Variables|Default|GetState)
      (:NewEnumerator1
        (Variables|難易度|SetAutoMoveElapsedTime (+ (Variables|難易度|GetAutoMoveElapsedTime) DeltaSeconds))
        (if (Variables|難易度|GetIsUpdateAutoMoveCount)
          ;[1 1 1] メンバーを衝突方向じゃないところに飛ばす
          (if (>= (Variables|難易度|GetAutoMoveElapsedTime) (Variables|難易度|GetAutoMoveInterval))
            (Variables|難易度|SetAutoMoveElapsedTime 0.0)
            (Physics|AddImpulse (Variables|Collision|GetCapsuleComponent) (Math|Vector|RotateVectorAroundAxis (* (Math|Vector|MakeVector 0.0 0.0 1.0) (Variables|難易度|GetAutoMoveStrength)) (Math|Random|RandomFloatinRange -45.0 45.0) "0,1.000000, 0") "None" true)))))))

(event Custom|OnAnimEnter
  (bind _output_get (Variables|アニメーション|SetNextState "NewEnumerator0"))
  (bind _output_get_2 (Variables|アニメーション|SetCurrentState _output_get))
  (bind _flipbook (CallFunction|GetAnim _output_get_2))
  (Sprite|SetFlipbook (Variables|Default|GetPaperFlipbook) _flipbook))

(event Custom|OnAnimChange
  (params (AnimType :type AnimType%20Enum))
  (Variables|アニメーション|SetNextState AnimType)
  (switch Utilities|FlowControl|Switch|SwitchonAnimType AnimType
    (:NewEnumerator0
      (if (not (Utilities|Enum|Equal(Enum) (Variables|アニメーション|GetCurrentState) "NewEnumerator1")) :!label _label ; beautifulさをやっているときはループが終わるまで待つ
        ;[1 1 1] 切り替え
        (bind _flipbook (CallFunction|GetAnim (Variables|アニメーション|GetNextState) :!label _label_2))
        (Sprite|SetFlipbook (Variables|Default|GetPaperFlipbook) _flipbook)
        (Variables|アニメーション|SetCurrentState (Variables|アニメーション|GetNextState))
        (Variables|アニメーション|SetPrevOffset "0, 0, 0")))
    (:NewEnumerator1
      (Utilities|FlowControl|Delay (Variables|アニメーション|GetTogetogeDelay))
      (Utilities|FlowControl|Sequence
        (:then_0
          ;[1 1 1] beautifulさのジャンプ
          (bind _localpos (Timeline|トゲトゲ移動 PlayFromStart)
            (:Update
              (Transformation|AddLocalOffset (Variables|Default|GetPaperFlipbook) (- _localpos (Variables|アニメーション|GetPrevOffset)) true true)
              (Variables|アニメーション|SetPrevOffset _localpos))
            (:LoopEvent
              (if (Utilities|Enum|NotEqual(Enum) (Variables|アニメーション|GetNextState) "NewEnumerator1") ; ここでAddLocalOffsetの誤差でずれそう
                (Utilities|FlowControl|Sequence
                  (:then_0
                    (Timeline|トゲトゲ移動 Stop))
                  (:then_1
                    (goto _label_2)))))))
        (:then_1
          (goto _label_2))))
    (:NewEnumerator2
      (goto _label))
    (:NewEnumerator3
      (goto _label))
    (:NewEnumerator5
      (goto _label))))

(event Custom|OnPauseAnim
  (bind _nextstate (Variables|アニメーション|GetNextState))
  ;[1 1 1] beautifulさのジャンプ
  (bind _localpos (Timeline|トゲトゲ移動 Stop)
    (:Update
      (Transformation|AddLocalOffset (Variables|Default|GetPaperFlipbook) (- _localpos (Variables|アニメーション|GetPrevOffset)) true true)
      (Variables|アニメーション|SetPrevOffset _localpos))
    (:LoopEvent
      (if (Utilities|Enum|NotEqual(Enum) _nextstate "NewEnumerator1") ; ここでAddLocalOffsetの誤差でずれそう
        (Utilities|FlowControl|Sequence
          (:then_0
            (Timeline|トゲトゲ移動 Stop))
          (:then_1
            ;[1 1 1] 切り替え
            (bind _flipbook (CallFunction|GetAnim _nextstate))
            (Sprite|SetFlipbook (Variables|Default|GetPaperFlipbook) _flipbook)
            (Variables|アニメーション|SetCurrentState _nextstate)
            (Variables|アニメーション|SetPrevOffset "0, 0, 0")))))))

(event Custom|OnResumeAnim
  (bind _nextstate (Variables|アニメーション|GetNextState))
  (if (Utilities|Enum|Equal(Enum) (Variables|アニメーション|GetCurrentState) "NewEnumerator1")
    ;[1 1 1] beautifulさのジャンプ
    (bind _localpos (Timeline|トゲトゲ移動 Play)
      (:Update
        (Transformation|AddLocalOffset (Variables|Default|GetPaperFlipbook) (- _localpos (Variables|アニメーション|GetPrevOffset)) true true)
        (Variables|アニメーション|SetPrevOffset _localpos))
      (:LoopEvent
        (if (Utilities|Enum|NotEqual(Enum) _nextstate "NewEnumerator1") ; ここでAddLocalOffsetの誤差でずれそう
          (Utilities|FlowControl|Sequence
            (:then_0
              (Timeline|トゲトゲ移動 Stop))
            (:then_1
              ;[1 1 1] 切り替え
              (bind _flipbook (CallFunction|GetAnim _nextstate))
              (Sprite|SetFlipbook (Variables|Default|GetPaperFlipbook) _flipbook)
              (Variables|アニメーション|SetCurrentState _nextstate)
              (Variables|アニメーション|SetPrevOffset "0, 0, 0"))))))))

(fn ConstructionScript
  (CallFunction|SetStageMode)
  (Variables|Default|SetStagePos (Transformation|GetActorLocation)))

(fn GetAnim
  (params (AnimType :type AnimType%20Enum))
  (bind _returnvalue (Math|Conversions|ToInteger(Byte) AnimType))
  (bind _idleflipbook (Variables|アニメーション|GetIdleFlipbook))
  (bind _togetogeflipbook (Variables|アニメーション|GetTogetogeFlipbook))
  (bind _specialflipbook (Variables|アニメーション|GetSpecialFlipbook))
  (bind _diveflipbook (Variables|アニメーション|GetDiveFlipbook))
  (bind _array (Utilities|Array|MakeArray _idleflipbook _togetogeflipbook _specialflipbook _diveflipbook))
  (if (> (Utilities|Array|Length _array) _returnvalue)
    (return (Utilities|Array|Get(acopy) _array _returnvalue))
    (elif (Utilities|Enum|Equal(Enum) AnimType "NewEnumerator5")
      ;[1 1 1] ダイブ中はアイドリングで代用
      (return (Variables|アニメーション|GetIdleFlipbook))
      (else
        ;[1 1 1] エラー
        (Development|PrintString "Index error")
        (return 0)))))

(fn IsTouched
  (bind _returnvalue (Game|GetPlayerController 0))
  (bind (_locationx _locationy) (Game|Player|GetMousePosition _returnvalue))
  (bind _returnvalue_2 (Math|Vector2D|MakeVector2D _locationx _locationy))
  (bind (_worldposition _worlddirection) (Class|GameplayStatics|DeprojectScreentoWorld _returnvalue _returnvalue_2))
  (bind _returnvalue_3 (Collision|LineTraceComponent (Variables|Collision|GetCapsuleComponent) _worldposition (+ _worldposition (* _worlddirection 1000)) false false))
  (return _returnvalue_3))

(fn SetPause
  (params (PauseEnabled :type Boolean))
  (bind _paperflipbook (Variables|Default|GetPaperFlipbook))
  (bind _output_get (Variables|Default|SetPauseEnabled PauseEnabled))
  (if _output_get
    (Audio|Components|Audio|Stop _paperflipbook)
    (else
      (Audio|Components|Audio|Play _paperflipbook))))

(fn StartSpecial
  (bind _manager (CallFunction|GetUnkoManager))
  (bind _activeunko (Default|GetActiveObjects _manager))
  (if (> (Utilities|Array|Length _activeunko) 0)
    (Utilities|Array|Clear (Variables|必殺技|GetTargets))
    (Physics|SetEnableGravity (Variables|Collision|GetCapsuleComponent) false)
    (Variables|必殺技|SetBeganSpecialTransform (Transformation|GetActorTransform))
    (Variables|必殺技|SetIsPlaySpecial true)
    (for _array_element _activeunko
      ;[1 1 1] todo : とりあえずインデックス順にしているけど近い順がいい
      (Utilities|Array|Add (Variables|必殺技|GetTargets) _array_element))
    (Variables|必殺技|SetCurrentTargetIndex 0)
    (CallFunction|SpecialMoveto (Utilities|Array|Get(acopy) (Variables|必殺技|GetTargets)))
    (Rendering|Material|SetMaterial (Variables|Default|GetPaperFlipbook) 0 "/Game/Characters/Members/Materials/MemberFrontMat.MemberFrontMat" :!pinned true) ; デプステストを切ったやつに差し替え\n（ステンシルテストがどこにあるか謎）
    (Rendering|SetTranslucentSortPriority (Variables|Default|GetPaperFlipbook) (CallFunction|GetRenderPriority "NewEnumerator5"))))

(fn StartDive
  (Variables|Default|SetState "NewEnumerator2")
  (Physics|SetEnableGravity (Variables|Collision|GetCapsuleComponent) true)
  (CallFunction|OnStartDive))

(fn UpdateDivingPosition
  (params (YRate :type Float%20%28single-precision%29) (Height :type Float%20%28single-precision%29) (MoveTo :type Vector))
  (if (> (Math|Vector|VectorLengthSquared (- MoveTo (Transformation|GetActorLocation))) 1e+03)
    (return (+ (+ (* (- MoveTo (Variables|Default|GetMoveBasePos)) YRate) (Math|Vector|MakeVector 0.0 0.0 Height)) (Variables|Default|GetMoveBasePos)))
    (else
      (return MoveTo))))

(fn SetDiveMode
  (bind _capsulecomponent (Variables|Collision|GetCapsuleComponent))
  (bind _capsulecomponent_2 (Variables|Collision|GetCapsuleComponent))
  (Class|PrimitiveComponent|SetConstraintMode _capsulecomponent "XZPlane")
  (Physics|SetEnableGravity _capsulecomponent true)
  (Transformation|SetActorTransform (Math|Transform|MakeTransform (Transformation|GetActorLocation) "0, 0, 0" (Transformation|GetActorScale3D))) ; 回転していたら元に戻す
  (CallFunction|OnAnimChange "NewEnumerator3")
  (Physics|SetSimulatePhysics _capsulecomponent_2 true)
  (Collision|SetCollisionEnabled _capsulecomponent_2 "QueryAndPhysics")
  (Variables|難易度|SetAutoMoveElapsedTime 0.0)
  (Variables|Default|SetState "NewEnumerator1"))

(fn SetStageMode
  (bind _capsulecomponent (Variables|Collision|GetCapsuleComponent))
  (Variables|Default|SetState "NewEnumerator0")
  (Class|PrimitiveComponent|SetConstraintMode _capsulecomponent "XZPlane")
  (Physics|SetEnableGravity _capsulecomponent false)
  (Rendering|SetTranslucentSortPriority (Variables|Default|GetPaperFlipbook) (CallFunction|GetRenderPriority "NewEnumerator3"))
  (CallFunction|OnAnimChange "NewEnumerator1"))

(fn EndSpecial
  (Physics|SetEnableGravity (Variables|Collision|GetCapsuleComponent) true)
  (Rendering|Material|SetMaterial (Variables|Default|GetPaperFlipbook) 0 "/Game/Characters/Members/Materials/MemberMat.MemberMat")
  (Rendering|SetTranslucentSortPriority (Variables|Default|GetPaperFlipbook) (CallFunction|GetRenderPriority "NewEnumerator0"))
  (Physics|SetSimulatePhysics (Variables|Collision|GetCapsuleComponent) true)
  (Variables|必殺技|SetIsPlaySpecial false))

(fn OnBeginSpecialCut
  (Physics|SetEnableGravity (Variables|Collision|GetCapsuleComponent) false)
  (Physics|SetSimulatePhysics (Variables|Collision|GetCapsuleComponent) false))

(fn ReturnStage
  (Variables|Default|SetState "NewEnumerator2")
  (Class|PrimitiveComponent|SetConstraintMode (Variables|Collision|GetCapsuleComponent) "Default")
  (Physics|SetSimulatePhysics (Variables|Collision|GetCapsuleComponent) false)
  (CallFunction|OnAnimChange "NewEnumerator5")
  (CallFunction|OnReturnStage))

(fn GetCurrentState
  (return (Variables|Default|GetState)))

(fn UpdateDivingRotation
  (params (InitialRotation :type Rotator))
  (Transformation|SetActorRotation (Math|Interpolation|RInterpTo InitialRotation (Math|Rotator|MakeRotator 0.0 0.0 0.0) (Utilities|Time|GetWorldDeltaSeconds) 0.5) true))