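; GameOverBG_BP is a game over background actor that shows a Paper2D sprite matching the current member.
; Shortly after BeginPlay, a brief delay leads into ApplyCurrentMember.
; That function looks up the member manager's current MemberType in the MemberSprites map and, if an entry exists, sets it on the sprite component.
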(event EventBeginPlay
  (Utilities|FlowControl|Delay 0.1)
  (CallFunction|ApplyCurrentMember))

(event Collision|EventActorBeginOverlap
  (params (OtherActor :type Actor%20Object%20Reference)))

(event EventTick
  (params (DeltaSeconds :type Float%20%28single-precision%29)))

(fn ConstructionScript)

(fn ApplyCurrentMember
  (bind _manager (CallFunction|GetMemberManager))
  (bind _membersprites (Variables|Default|GetMemberSprites))
  (bind _currentmember (Variables|/Game/Blueprints/Members/MemberManager.MemberManager_C|GetCurrentMember _manager))
  (bind _membertype (Variables|/Game/Blueprints/Members/MemberBase_BP.MemberBase_BP_C|GetMemberType _currentmember))
  (bind (_value _returnvalue) (Utilities|Map|Find _membersprites _membertype))
  (if _returnvalue
    (Rendering|Components|Sprite|SetSprite (Variables|Default|GetPaperSprite) _value)))